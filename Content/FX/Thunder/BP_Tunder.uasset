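; Blueprint for a thunder strike effect that fires at random intervals while IsInTrigger is set.
; Tick runs through a random Delay to space out strikes, then calls Strike and briefly pulses the Skylight intensity for a flash.
; Strike plays the Thunder_Strike timeline, whose Y track drives the "Y" and scaled "emission" material parameters on BPThunderPlane.
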(event Custom|Strike
  (bind _bp_thunder_plane (Variables|Default|GetBP_Thunder_plane))
  (bind _y (Timeline|Thunder_Strike PlayFromStart)
    (:Update
      (Rendering|Material|SetScalarParameterValueonMaterials _bp_thunder_plane "Y" _y)
      (Rendering|Material|SetScalarParameterValueonMaterials _bp_thunder_plane "emission" (* (+ _y 0.0) -1e+02)))))

(event EventBeginPlay)

(event EventTick
  (params (DeltaSeconds :type Float%20%28single-precision%29))
  (bind _skylight (Variables|Default|Getskylight))
  (bind _lightcomponent (Variables|/Script/Engine.SkyLight|GetLightComponent _skylight))
  (Utilities|FlowControl|Delay (Math|Random|RandomFloatinRange 4.0 1e+01))
  (if (Variables|Default|GetIsInTrigger)
    (CallFunction|Strike)
    (Utilities|FlowControl|Delay 0.1)
    (Rendering|Components|Light|SetIntensity _lightcomponent 15.0)
    (Utilities|FlowControl|Delay 0.15)
    (Rendering|Components|Light|SetIntensity _lightcomponent 0.0)))

(fn ConstructionScript)